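; BP_Lander is a player-controlled lander pawn flown with physics thrusters.
; The ThrustUp axis scales the strength of four upward thrusters together, while ThrustRight drives a separate thruster scaled by a rotation multiplier.
; BeginPlay stores a vector derived from the starting rotation for resetting, but the ResetPlayer event triggered by input is empty and the reset-location assignment is disconnected.
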(event Custom|Reset%20Player)

(event EventBeginPlay
  (Variables|Default|SetResetRot (Math|Rotator|GetRotationXVector (Transformation|GetActorRotation))))

(event Input|ActionEvents|InputActionResetPlayer
  (params (Key :type Key%20Structure))
  (:Pressed
    (CallFunction|ResetPlayer)))

(event Input|AxisEvents|InputAxisThrustUp
  (params (AxisValue :type Float%20%28single-precision%29))
  ;[1 1 1] Physics
  ;;[1 1 1] Upwards Thrust
  (for _array_element (Utilities|Array|MakeArray (Variables|Default|GetPhysicsThruster) (Variables|Default|GetPhysicsThruster1) (Variables|Default|GetPhysicsThruster2) (Variables|Default|GetPhysicsThruster3))
    (Variables|/Script/Engine.PhysicsThrusterComponent|SetThrustStrength _array_element (* AxisValue (Variables|Default|GetUpward%20Thrust%20Strenght)))))

(event Input|AxisEvents|InputAxisThrustRight
  (params (AxisValue :type Float%20%28single-precision%29))
  ;[1 1 1] Physics
  ;;[1 1 1] Rigth Thrust
  (Variables|/Script/Engine.PhysicsThrusterComponent|SetThrustStrength (Variables|Default|GetPhysicsThrusterR) (* AxisValue (Variables|Default|GetRotate%20Multiplier))))

(fn ConstructionScript)